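; BP_Player is the player character Blueprint that sets up Enhanced Input and handles movement.
; On BeginPlay it casts its controller to BP_CharacterController and adds the IMC_Player mapping context to that player's input subsystem.
; IA_Move drives movement input along fixed world right and forward vectors rather than control rotation, and prints the X axis value as debug output.
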(event Input|EnhancedActionEvents|EnhancedInputActionIA_Move
  (params (ActionValue :type Vector%202D%20Structure) (ElapsedSeconds :type Float%20%28double-precision%29) (TriggeredSeconds :type Float%20%28double-precision%29) (InputAction :type Input%20Action%20Object%20Reference :default "/Game/Character/Input/Actions/IA_Move.IA_Move"))
  ;[1 1 1] Movement
  (Development|PrintString (Utilities|String|ToString(Float) (.x ActionValue)))
  (Pawn|Input|AddMovementInput (Class|KismetMathLibrary|VectorRight) (.x ActionValue) false)
  (Pawn|Input|AddMovementInput (Class|KismetMathLibrary|VectorForward) (.y ActionValue) false))

(event EventBeginPlay
  (bind _asbp_character_controller (Utilities|Casting|CastToBP_CharacterController (Pawn|GetController)))
  (Input|AddMappingContext (PlayerController|LocalPlayerSubsystems|GetEnhancedInputLocalPlayerSubsystem _asbp_character_controller) "/Game/Character/Input/IMC_Player.IMC_Player" 0 "(bIgnoreAllPressedKeysUntilRelease=True,bForceImmediately=False,bNotifyUserSettings=False)"))

(fn ConstructionScript)