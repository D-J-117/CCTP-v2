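; BP_MainCam is a camera Blueprint that provides an orthographic view.
; On BeginPlay it activates its camera and scene components, then switches the camera to orthographic projection with a fixed, wide ortho width.
; The construction script is empty, and a post-process settings node sits unconnected, so it never runs.
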(event EventBeginPlay
  (bind _self self)
  (bind _self_2 self)
  (bind _cameracomponent (Variables|CameraActor|GetCameraComponent _self))
  (Components|Activation|SetActive (Variables|CameraActor|GetCameraComponent _self_2) true false)
  (Components|Activation|SetActive (Variables|Default|GetSceneComponent _self_2) true false)
  (Class|CameraComponent|SetProjectionMode _cameracomponent "Orthographic")
  (Class|CameraComponent|SetOrthoWidth _cameracomponent 4096.0))

(fn ConstructionScript)