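; Learning Agents reinforcement learning trainer that teaches BP_CharacterAgent to move quickly along the level's BP_TrackSpline without leaving the track.
; Rewards velocity along the spline and penalizes planar distance from the nearest spline point beyond a threshold, using a spline helper for both.
; A wider off-track threshold completes the episode.
; Episode resets send each agent to a random point on the spline, which is cached at BeginPlay.
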(event EventSetupRewards
  ;[1 1 1] For this tutorial, we want the agent to drive as fast as possible around the track and we want them to stay on the track. We add a reward for speed along the spline and a penalty for leaving the track.
  (Utilities|FlowControl|Sequence
    (:then_0
      (bind _returnvalue (Class|PlanarPositionDifferencePenalty|AddPlanarPositionDifferencePenalty 0 "OffTrackPenalty" 1.0 1e+02 8e+02 "1.000000,0.000000,0.000000" "0.000000,1.000000,0.000000"))
      (Variables|Default|SetOffTrackPenalty _returnvalue))
    (:then_1
      (bind _returnvalue_2 (Class|ScalarVelocityReward|AddScalarVelocityReward 0 "SpeedReward" 0.1 2e+02))
      (Variables|Default|SetVelocityAlongTrackReward _returnvalue_2))
    (:then_2
      (bind _returnvalue_3 (Class|SplineComponentHelper|AddSplineComponentHelper 0 "SplineComponentRewardHelper"))
      (Variables|Default|SetSplineComponentRewardHelper _returnvalue_3))))

(event EventSetRewards
  (params (AgentIds :type Array%20of%20Integers))
  ;[1 1 1] Gathers the speed along the spline and penalties for leaving the track
  (for _array_element AgentIds
    (Utilities|FlowControl|Sequence
      (:then_0
        (bind _returnvalue (Class|SplineComponentHelper|GetNearestPositiononSpline (Variables|Default|GetSplineComponentRewardHelper) _array_element (Variables|Default|GetTrack%20Spline) (Transformation|GetActorLocation (Class|LearningAgentsManagerComponent|GetAgent _array_element "/Game/Learning/BP_CharacterAgent.BP_CharacterAgent_C")) "World"))
        (Class|PlanarPositionDifferencePenalty|SetPlanarPositionDifferencePenalty (Variables|Default|GetOffTrackPenalty) _array_element _returnvalue (Transformation|GetActorLocation (Class|LearningAgentsManagerComponent|GetAgent _array_element "/Game/Learning/BP_CharacterAgent.BP_CharacterAgent_C"))))
      (:then_1
        (bind _returnvalue_2 (Class|SplineComponentHelper|GetVelocityAlongSpline (Variables|Default|GetSplineComponentRewardHelper) _array_element (Variables|Default|GetTrack%20Spline) (Transformation|GetActorLocation (Class|LearningAgentsManagerComponent|GetAgent _array_element "/Game/Learning/BP_CharacterAgent.BP_CharacterAgent_C")) (Transformation|GetVelocity (Class|LearningAgentsManagerComponent|GetAgent _array_element "/Game/Learning/BP_CharacterAgent.BP_CharacterAgent_C")) 1e+01 "World"))
        (Class|ScalarVelocityReward|SetScalarVelocityReward (Variables|Default|GetVelocityAlongTrackReward) _array_element _returnvalue_2)))))

(event EventBeginPlay
  (bind _returnvalue (Actor|GetActorOfClass "/Game/Learning/BP_TrackSpline.BP_TrackSpline_C"))
  (Variables|Default|SetTrack%20Spline (Variables|/Game/Learning/BP_TrackSpline.BP_TrackSpline_C|GetSpline _returnvalue)))

(event EventSetupCompletions
  ;[1 1 1] Setting up completion conditions
  (bind _returnvalue (Class|PlanarPositionDifferenceCompletion|AddPlanarPositionDifferenceCompletion 0 "OffTrackCompletion" 1.2e+03 "Termination" "1.000000,0.000000,0.000000" "0.000000,1.000000,0.000000"))
  (Variables|Default|SetOffTrackTermination _returnvalue))

(event EventResetEpisodes
  (params (AgentIds :type Array%20of%20Integers))
  ;[1 1 1] Resets Agent position upon completion
  (for _array_element AgentIds
    (Default|ResettoRandonPointonSpline (Class|LearningAgentsManagerComponent|GetAgent _array_element "/Game/Learning/BP_CharacterAgent.BP_CharacterAgent_C") (Variables|Default|GetTrack%20Spline))))

(event EventSetCompletions
  (params (AgentIds :type Array%20of%20Integers))
  ;[1 1 1] Setting up completion conditions
  (for _array_element AgentIds
    (bind _returnvalue (Class|SplineComponentHelper|GetNearestPositiononSpline (Variables|Default|GetSplineComponentRewardHelper) _array_element (Variables|Default|GetTrack%20Spline) (Transformation|GetActorLocation (Class|LearningAgentsManagerComponent|GetAgent _array_element "/Game/Learning/BP_CharacterAgent.BP_CharacterAgent_C")) "World"))
    (Class|PlanarPositionDifferenceCompletion|SetPlanarPositionDifferenceCompletion (Variables|Default|GetOffTrackTermination) _array_element _returnvalue (Transformation|GetActorLocation (Class|LearningAgentsManagerComponent|GetAgent _array_element "/Game/Learning/BP_CharacterAgent.BP_CharacterAgent_C")))))