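; BP_RLTrainingManager drives reinforcement learning training of a movement policy using Learning Agents.
; On BeginPlay it sets up the moving interactor, then the policy with that interactor and the DA_MovementNetwork asset, then the trainer with both.
; Each Tick calls RunTraining without reinitializing the policy network.
; The Tick interval is raised to 0.1s so each action has time to affect the game state.
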(event EventBeginPlay
  ;[1 1 1] Call each component's setup function
  (Utilities|FlowControl|Sequence
    (:then_0
      (Class|LearningAgentsInteractor|SetupInteractor (Variables|Default|GetBP_MovingInteractor)))
    (:then_1
      (Class|LearningAgentsPolicy|SetupPolicy (Variables|Default|GetBP_MovementPolicy) (Variables|Default|GetBP_MovingInteractor) (Variables|Default|GetPolicy%20Settings) "/Game/Learning/DA_MovementNetwork.DA_MovementNetwork"))
    (:then_2
      (Class|LearningAgentsTrainer|SetupTrainer (Variables|Default|GetBP_MovementRLTrainer) (Variables|Default|GetBP_MovingInteractor) (Variables|Default|GetBP_MovementPolicy) 0 (Variables|Default|GetTrainer%20Settings)))))

(event EventTick
  (params (DeltaSeconds :type Float%20%28single-precision%29))
  ;[1 1 1] Running the training step each tick. We have increatsed the Tick Interval of this blueprint to 0.1s to allow some time to pass in order for the action to have time to affect the game state.
  (Class|LearningAgentsTrainer|RunTraining (Variables|Default|GetBP_MovementRLTrainer) (Variables|Default|GetTrainer%20Training%20Settings) (Variables|Default|GetTrainer%20Game%20Settings) (Variables|Default|GetTrainer%20Path%20Settings) (Variables|Default|GetCritic%20Settings) false true true))

(fn ConstructionScript)