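; Character agent that registers with the Learning Agents manager on BeginPlay, storing its ID for learning.
; Enhanced Input drives yaw and forward movement, and attacks spawn projectiles from limited ammo that Tick refills after delays; damage briefly flashes a red overlay.
; A reset function teleports it near a random spline point with randomized yaw and zeroed mesh velocities.
; The controller cast and mapping-context setup are unwired, leaving the controller reference used for turning unset here.
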(event Custom|TakeDamage
  (Rendering|Material|SetOverlayMaterial (Variables|Default|GetCube) "/Game/Materials/MI_RedTransparent.MI_RedTransparent" :!class /Script/Engine.MeshComponent)
  (Utilities|FlowControl|Delay 1.0)
  (Rendering|Material|SetOverlayMaterial (Variables|Default|GetCube) 0 :!class /Script/Engine.MeshComponent))

(event Custom|AttackEvent
  (bind _returnvalue (Transformation|GetActorTransform))
  (bind (_location _rotation _scale) (Math|Transform|BreakTransform _returnvalue))
  (if (> (Variables|Default|GetCurrent%20Ammo) 0)
    (Game|SpawnActorfromClass "/Game/Character/BP_Projectile.BP_Projectile_C" (Math|Transform|MakeTransform (+ (* (Transformation|GetActorForwardVector) 2e+02) _location) _rotation _scale) "AlwaysSpawn" "MultiplyWithRoot" 0 0)
    (Math|Integer|DecrementInt (Variables|Default|GetCurrent%20Ammo))))

(event Input|EnhancedActionEvents|EnhancedInputActionIA_Move
  (params (ActionValue :type Vector%202D%20Structure) (ElapsedSeconds :type Float%20%28double-precision%29) (TriggeredSeconds :type Float%20%28double-precision%29) (InputAction :type Input%20Action%20Object%20Reference :default "/Game/Character/Input/Actions/IA_Move.IA_Move"))
  (bind _as_bp_character_controller (Variables|Default|GetAs%20BP%20Character%20Controller))
  (bind _returnvalue (Pawn|GetControlRotation _as_bp_character_controller :!class /Script/Engine.Controller))
  ;[1 1 1] Movement
  (Pawn|SetControlRotation (Pawn|GetController) (Math|Rotator|MakeRotator (.roll _returnvalue) (.pitch _returnvalue) (+ (.yaw _returnvalue) (* 1.0 (.x ActionValue)))))
  (Pawn|Input|AddMovementInput (Transformation|GetActorForwardVector) (.y ActionValue) false))

(event Input|EnhancedActionEvents|EnhancedInputActionIA_Attack
  (params (ActionValue :type Boolean) (ElapsedSeconds :type Float%20%28double-precision%29) (TriggeredSeconds :type Float%20%28double-precision%29) (InputAction :type Input%20Action%20Object%20Reference :default "/Game/Character/Input/Actions/IA_Attack.IA_Attack"))
  (:Started
    (CallFunction|AttackEvent)))

(event EventTick
  (params (DeltaSeconds :type Float%20%28single-precision%29))
  (if (< (Variables|Default|GetCurrent%20Ammo) 3)
    (Utilities|FlowControl|Delay 1.0)
    (Math|Integer|IncrementInt (Variables|Default|GetCurrent%20Ammo))))

(event EventBeginPlay
  ;[1 1 1] Register agents with Manager
  (|CallParentFunction)
  (bind _returnvalue (Actor|GetActorOfClass "/Script/LearningAgents.LearningAgentsManager"))
  (Utilities|IsValid _returnvalue
    (:Is%20Valid
      (bind _returnvalue_2 (Class|LearningAgentsManager|AddAgent _returnvalue self))
      (Variables|Default|SetAgent%20Id _returnvalue_2))
    (:Is%20Not%20Valid
      (Development|PrintString "Could not find Learning Agents manager. "))))

(fn ConstructionScript)

(fn ResettoRandonPointonSpline
  (params (Spline :type Spline%20Component%20Object%20Reference))
  (bind _returnvalue (Spline|GetSplineLength Spline))
  (bind _returnvalue_2 (Math|Random|RandomFloat))
  (bind _mesh (Variables|Character|GetMesh))
  (bind _returnvalue_3 (* _returnvalue_2 _returnvalue))
  (Transformation|SetActorTransform (Math|Transform|MakeTransform (+ (Math|Vector|MakeVector (* (- (Math|Random|RandomFloat) 0.5) 1.2e+03) (* (- (Math|Random|RandomFloat) 0.5) 1.2e+03) 5e+01) (Spline|GetLocationatDistanceAlongSpline Spline _returnvalue_3 "World")) (Math|Rotator|MakeRotator 0.0 0.0 (+ (.Yaw (Math|Rotator|BreakRotator (Spline|GetRotationatDistanceAlongSpline Spline _returnvalue_3 "World"))) (* (- (Math|Random|RandomFloat) 0.5) 9e+01)))) false true)
  (Class|PrimitiveComponent|SetPhysicsAngularVelocityinDegrees _mesh "0, 0, 0" false "None") ; Interrupt any angular movement
  (Physics|SetPhysicsLinearVelocity _mesh "0, 0, 0" false "None") ; Interrupt any linear movement
)