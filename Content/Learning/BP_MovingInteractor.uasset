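; Learning Agents interactor that lets BP_CharacterAgent characters observe and follow a BP_TrackSpline track.
; Observations take the nearest spline distance to derive track position, direction and lap-progress angle, plus agent velocity, mostly agent-relative.
; Two float actions drive each agent: the throttle's sign alone triggers full forward or backward movement input, while steering adds directly to controller yaw.
; Disconnected goal-location observation nodes never run.
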(event EventGetActions
  (params (AgentIds :type Array%20of%20Integers))
  ;[1 1 1] We take the values from the neural network and apply them to the Agent
  (for _array_element AgentIds
    (Utilities|FlowControl|Sequence
      (:then_0
        ;[1 1 1] Fowards/Backwards Movement
        (bind _returnvalue (Class|FloatAction|GetFloatAction (Variables|Actions|GetForwardsBackwardsAction) _array_element))
        (if (> _returnvalue 0.0)
          (Pawn|Input|AddMovementInput (Class|LearningAgentsManagerComponent|GetAgent _array_element "/Game/Learning/BP_CharacterAgent.BP_CharacterAgent_C") (Transformation|GetActorForwardVector (Class|LearningAgentsManagerComponent|GetAgent _array_element "/Game/Learning/BP_CharacterAgent.BP_CharacterAgent_C")) 1.0 false)
          (elif (< _returnvalue 0.0)
            (Pawn|Input|AddMovementInput (Class|LearningAgentsManagerComponent|GetAgent _array_element "/Game/Learning/BP_CharacterAgent.BP_CharacterAgent_C") (* (Transformation|GetActorForwardVector (Class|LearningAgentsManagerComponent|GetAgent _array_element "/Game/Learning/BP_CharacterAgent.BP_CharacterAgent_C")) -1) 1.0 false))))
      (:then_1
        ;[1 1 1] Turning and Rotation
        (bind _returnvalue_2 (Class|FloatAction|GetFloatAction (Variables|Actions|GetSteeringAction) _array_element))
        (Pawn|SetControlRotation (Pawn|GetController (Class|LearningAgentsManagerComponent|GetAgent _array_element "/Game/Learning/BP_CharacterAgent.BP_CharacterAgent_C")) (Math|Rotator|MakeRotator (.roll (Pawn|GetControlRotation (Pawn|GetController (Class|LearningAgentsManagerComponent|GetAgent _array_element "/Game/Learning/BP_CharacterAgent.BP_CharacterAgent_C")) :!class /Script/Engine.Controller)) (.pitch (Pawn|GetControlRotation (Pawn|GetController (Class|LearningAgentsManagerComponent|GetAgent _array_element "/Game/Learning/BP_CharacterAgent.BP_CharacterAgent_C")) :!class /Script/Engine.Controller)) (+ (.yaw (Pawn|GetControlRotation (Pawn|GetController (Class|LearningAgentsManagerComponent|GetAgent _array_element "/Game/Learning/BP_CharacterAgent.BP_CharacterAgent_C")) :!class /Script/Engine.Controller)) (* 1.0 _returnvalue_2))))))))

(event EventSetupObservations
  ;[1 1 1] Setup for all observations that the Agent needs to make. Based on tutorial listed above.
  (Utilities|FlowControl|Sequence
    (:then_0
      (bind _returnvalue (Class|PlanarPositionObservation|AddPlanarPositionObservation 0 "TrackPositionObservation" 1e+02 "1.000000,0.000000,0.000000" "0.000000,1.000000,0.000000"))
      (Variables|Observations|SetTrackPositionObservation _returnvalue)
      (bind _returnvalue_2 (Class|PlanarDirectionObservation|AddPlanarDirectionObservation 0 "TrackDirectionObservation" 1.0 "1.000000,0.000000,0.000000" "0.000000,1.000000,0.000000"))
      (Variables|Observations|SetTrackDirectionObservation _returnvalue_2))
    (:then_1
      (bind _returnvalue_3 (Class|AngleObservation|AddAngleObservation 0 "TrackGlobalPositionObservation" 1.0))
      (Variables|Observations|SetTrackGlobalPositionObservation _returnvalue_3)
      (bind _returnvalue_4 (Class|PlanarVelocityObservation|AddPlanarVelocityObservation 0 "CarVelocityObservation" 2e+02 "1.000000,0.000000,0.000000" "0.000000,1.000000,0.000000"))
      (Variables|Observations|SetCarVelocityObservation _returnvalue_4))
    (:then_2
      (bind _returnvalue_5 (Class|SplineComponentHelper|AddSplineComponentHelper 0 "SplineComponentHelper"))
      (Variables|Observations|SetSplineComponentHelper _returnvalue_5)
      (bind _returnvalue_6 (Actor|GetActorOfClass "/Game/Learning/BP_TrackSpline.BP_TrackSpline_C"))
      (Variables|Default|SetTrackSpline (Variables|/Game/Learning/BP_TrackSpline.BP_TrackSpline_C|GetSpline _returnvalue_6)))))

(event EventSetObservations
  (params (AgentIds :type Array%20of%20Integers))
  ;[1 1 1] Assigns values to all observations
  (for _array_element AgentIds
    (bind _returnvalue (Class|SplineComponentHelper|GetDistanceAlongSplineatPosition (Variables|Observations|GetSplineComponentHelper) _array_element (Variables|Default|GetTrackSpline) (Transformation|GetActorLocation (Class|LearningAgentsManagerComponent|GetAgent _array_element "/Game/Learning/BP_CharacterAgent.BP_CharacterAgent_C")) "World"))
    (Utilities|FlowControl|Sequence
      (:then_0
        (bind _returnvalue_2 (Class|SplineComponentHelper|GetPositionatDistanceAlongSpline (Variables|Observations|GetSplineComponentHelper) _array_element (Variables|Default|GetTrackSpline) _returnvalue "World"))
        (Class|PlanarPositionObservation|SetPlanarPositionObservation (Variables|Observations|GetTrackPositionObservation) _array_element _returnvalue_2 (Transformation|GetActorLocation (Class|LearningAgentsManagerComponent|GetAgent _array_element "/Game/Learning/BP_CharacterAgent.BP_CharacterAgent_C")) (Transformation|GetActorRotation (Class|LearningAgentsManagerComponent|GetAgent _array_element "/Game/Learning/BP_CharacterAgent.BP_CharacterAgent_C"))))
      (:then_1
        (bind _returnvalue_3 (Class|SplineComponentHelper|GetDirectionatDistanceAlongSpline (Variables|Observations|GetSplineComponentHelper) _array_element (Variables|Default|GetTrackSpline) _returnvalue "World"))
        (Class|PlanarDirectionObservation|SetPlanarDirectionObservation (Variables|Observations|GetTrackDirectionObservation) _array_element _returnvalue_3 (Transformation|GetActorRotation (Class|LearningAgentsManagerComponent|GetAgent _array_element "/Game/Learning/BP_CharacterAgent.BP_CharacterAgent_C"))))
      (:then_2
        (bind _returnvalue_4 (Class|SplineComponentHelper|GetProportionAlongSplineasAngle (Variables|Observations|GetSplineComponentHelper) _array_element (Variables|Default|GetTrackSpline) _returnvalue))
        (Class|AngleObservation|SetAngleObservation (Variables|Observations|GetTrackGlobalPositionObservation) _array_element _returnvalue_4 0.0))
      (:then_3
        (Class|PlanarVelocityObservation|SetPlanarVelocityObservation (Variables|Observations|GetCarVelocityObservation) _array_element (Transformation|GetVelocity (Class|LearningAgentsManagerComponent|GetAgent _array_element "/Game/Learning/BP_CharacterAgent.BP_CharacterAgent_C")) (Transformation|GetActorRotation (Class|LearningAgentsManagerComponent|GetAgent _array_element "/Game/Learning/BP_CharacterAgent.BP_CharacterAgent_C")))))))

(event EventSetupActions
  ;[1 1 1] Declares the actions that Agents can perform.
  (Utilities|FlowControl|Sequence
    (:then_0
      (bind _returnvalue (Class|FloatAction|AddFloatAction 0 "ForwardsBackwardsAction" 1.0))
      (Variables|Actions|SetForwardsBackwardsAction _returnvalue))
    (:then_1
      (bind _returnvalue_2 (Class|FloatAction|AddFloatAction 0 "SteeringAction" 1.0))
      (Variables|Actions|SetSteeringAction _returnvalue_2))))